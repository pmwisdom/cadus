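; Enemy turret actor that fires lasers and can be destroyed by damage.
; Tick spawns a Laser actor at the ProjectileSpawn transform every frame, with no cooldown or targeting.
; AffectHealth passes the health delta to the ActorStatus component and prints the current health.
; When ActorStatus reports death, a large explosion particle effect spawns at the Cylinder's location and the turret destroys itself.
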(event EventBeginPlay)

(event Collision|EventActorBeginOverlap
  (params (OtherActor :type Actor%20Object%20Reference)))

(event EventTick
  (params (DeltaSeconds :type Float%20%28single-precision%29))
  (Game|SpawnActorfromClass "/Game/Blueprints/Laser.Laser_C" (Transformation|GetWorldTransform (Variables|Default|GetProjectileSpawn)) "Undefined" 0 0))

(event EventAffectHealth
  (params (Delta :type Integer))
  (bind _actorstatus (Variables|Default|GetActorStatus))
  (Class|ActorStatus|DamageActor (Variables|Default|GetActorStatus) Delta)
  (Development|PrintString (Utilities|String|ToString(Integer) (Variables|/Script/Cadus.ActorStatus|GetCurrentHealth _actorstatus)))
  (if (Variables|/Script/Cadus.ActorStatus|GetbIsDead _actorstatus)
    (Effects|SpawnEmitteratLocation "/Game/StarterContent/Particles/P_Explosion_BIG.P_Explosion_BIG" (Transformation|GetWorldLocation (Variables|Default|GetCylinder)))
    (Actor|DestroyActor)))

(fn ConstructionScript)