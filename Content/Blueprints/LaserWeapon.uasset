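; Laser weapon Blueprint that spawns Laser actors at its ProjectileSpawnPoint transform.
; PullTrigger passes through a DoOnce gate to fire immediately, then sets a timer by function name to call Fire after an interval derived from RoundsPerSecond.
; ReleaseTrigger clears that timer and resets the gate for the next pull.
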(event Custom|PullTrigger
  (Utilities|FlowControl|DoOnce false
    (:Completed
      (CallFunction|Fire)
      (Utilities|Time|SetTimerbyFunctionName 0 "Fire" (/ 1.0 (Variables|Default|Getrounds%20per%20second))))))

(event Custom|ReleaseTrigger
  (Utilities|Time|ClearTimerbyFunctionName 0 "Fire")
  (Utilities|FlowControl|DoOnce false) ; enters at Reset
)

(event Custom|Fire
  (Game|SpawnActorfromClass "/Game/Blueprints/Laser.Laser_C" (Transformation|GetWorldTransform (Variables|Default|GetProjectileSpawnPoint)) "Undefined" 0 0))

(fn ConstructionScript)