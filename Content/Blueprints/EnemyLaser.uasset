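; EnemyLaser is a laser projectile fired by enemies that damages what it hits.
; On overlap, damageable actors without the Enemy tag receive its Damage through the IDamageable health message, and the laser then explodes.
; Damageable enemies are passed through untouched, while any non-damageable actor also triggers the explosion.
; The explosion spawns a particle emitter at the laser's location and destroys the actor.
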(event Custom|Destroy%20And%20Emit
  (Effects|SpawnEmitteratLocation "/Game/StarterContent/Particles/P_Explosion.P_Explosion" (Transformation|GetActorLocation))
  (Actor|DestroyActor))

(event EventBeginPlay)

(event Collision|EventActorBeginOverlap
  (params (OtherActor :type Actor%20Object%20Reference))
  (if (Utilities|DoesObjectImplementInterface OtherActor "/Game/Blueprints/iDamageable.iDamageable_C")
    (if (not (Actor|ActorHasTag OtherActor "Enemy"))
      (Class|IDamageable|AffectHealth(Message) OtherActor (Variables|Default|GetDamage))
      (CallFunction|DestroyandEmit))
    (else
      (CallFunction|DestroyandEmit))))

(fn ConstructionScript)